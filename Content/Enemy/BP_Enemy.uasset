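; BP_Enemy is an enemy pawn that runs the BT_Enemy behavior tree and takes damage from the player's sword.
; On spawn it seeds the blackboard's TargetDestination with a fixed point, and heard noise from a character triggers a direct AI move toward that character.
; A capsule overlap with Weapon_Sword while the player is slashing subtracts Health on MyHealthComponent and destroys the enemy at zero.
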(event OnComponentBeginOverlap(CapsuleComponent)
  (params (OverlappedComponent :type Primitive%20Component%20Object%20Reference) (OtherActor :type Actor%20Object%20Reference) (OtherComp :type Primitive%20Component%20Object%20Reference) (OtherBodyIndex :type Integer) (bFromSweep :type Boolean) (SweepResult :type Hit%20Result%20Structure%20%28by%20ref%29))
  (Utilities|Casting|CastToWeapon_Sword OtherActor)
  (bind _astop_down_character (Utilities|Casting|CastToTopDownCharacter (Game|GetPlayerCharacter 0)))
  (if (Variables|/Game/TopDownCPP/Blueprints/TopDownCharacter.TopDownCharacter_C|GetSlashing%20Sword _astop_down_character)
    (Development|PrintString "HIt By Sword")
    (bind _asmy_health_component (Utilities|Casting|CastToMyHealthComponent (Actor|GetComponentbyClass "/Script/testing.MyHealthComponent")))
    (bind _output_get (Variables|/Script/testing.MyHealthComponent|SetHealth _asmy_health_component (- (Variables|/Script/testing.MyHealthComponent|GetHealth _asmy_health_component) 2e+01)))
    (if (<= _output_get 0.0)
      (Development|PrintString "Killed")
      (Actor|DestroyActor))))

(event OnHearNoise(PawnSensing)
  (params (Instigator :type Pawn%20Object%20Reference) (Location :type Vector%20%28by%20ref%29 :default "0, 0, 0") (Volume :type Float%20%28single-precision%29))
  (bind _ascharacter (Utilities|Casting|CastToCharacter Instigator))
  (AI|AIMoveTo self "0, 0, 0" _ascharacter 5.0 false))

(event EventBeginPlay
  (AI|RunBehaviorTree (AI|GetAIController self) "/Game/Enemy/BT_Enemy.BT_Enemy")
  (AI|Components|Blackboard|SetValueasVector (AI|GetBlackboard self) (Utilities|Name|MakeLiteralName "TargetDestination") "-800.000000,-800.000000,170.000000"))

(fn ConstructionScript)